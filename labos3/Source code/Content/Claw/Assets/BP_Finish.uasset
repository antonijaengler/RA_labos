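; BP_Finish is the drop-off trigger in the claw game that scores whatever actor overlaps it.
; On overlap it destroys that actor without filtering, sets the Empty flag on player 0's BP_ClawCharacter_Test, then calls AddScore on ClawGameMode.
; A delayed FinishGame call on the game mode is left disconnected and never runs.
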(event EventBeginPlay)

(event Collision|EventActorBeginOverlap
  (params (OtherActor :type Actor%20Object%20Reference))
  (Actor|DestroyActor OtherActor)
  (bind _asbp_claw_character_test (Utilities|Casting|CastToBP_ClawCharacter_Test (Game|GetPlayerCharacter 0)))
  (Variables|/Game/Claw/BP_ClawCharacter_Test.BP_ClawCharacter_Test_C|SetEmpty _asbp_claw_character_test true)
  (bind _asclaw_game_mode (Utilities|Casting|CastToClawGameMode (Game|GetGameMode)))
  (Default|AddScore _asclaw_game_mode))

(event EventTick
  (params (DeltaSeconds :type Float%20%28single-precision%29)))

(fn ConstructionScript)