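; Test claw character Blueprint that lets the player move a Control Rig control with input axes and look around via controller yaw and pitch.
; Movement axes set scaled X/Y/Z offsets, added to Control_ctrl's local position before each forwards solve.
; The ControlRig component maps the complete skeletal mesh on pre-initialize, and the construction script copies the mesh's relative rotation onto it.
; The Exit action quits the game.
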(event OnPreForwardsSolveDelegate(ControlRig)
  (params (Component :type Control%20Rig%20Component%20Object%20Reference))
  (bind _controlrig (Variables|Default|GetControlRig))
  ;[1 1 1] Control Rig logic
  (Class|ControlRigComponent|SetControlPosition _controlrig "Control_ctrl" (+ (Class|ControlRigComponent|GetControlPosition _controlrig "Control_ctrl" "LocalSpace") (Math|Vector|MakeVector (Variables|Default|GetOffsetX) (Variables|Default|GetoffsetY) (Variables|Default|GetOffsetZ))) "LocalSpace"))

(event OnPreInitializeDelegate(ControlRig)
  (params (Component :type Control%20Rig%20Component%20Object%20Reference))
  ;[1 1 1] Control Rig logic
  (Class|ControlRigComponent|AddMappedCompleteSkeletalMesh Component))

(event EventBeginPlay
  (Variables|Default|SetEmpty true))

(event Collision|EventActorBeginOverlap
  (params (OtherActor :type Actor%20Object%20Reference)))

(event EventTick
  (params (DeltaSeconds :type Float%20%28single-precision%29)))

(event Input|ActionEvents|InputActionExit
  (params (Key :type Key%20Structure :default "None"))
  (:Pressed
    (Game|QuitGame 0 "Quit" false)))

(event Input|AxisEvents|InputAxisMoveForwardBackward
  (params (AxisValue :type Float%20%28single-precision%29))
  ;[1 1 1] Movement Logic
  (Variables|Default|SetOffsetX (* AxisValue 1e+01)))

(event Input|AxisEvents|InputAxisMoveLeftRight
  (params (AxisValue :type Float%20%28single-precision%29))
  ;[1 1 1] Movement Logic
  (Variables|Default|SetoffsetY (* AxisValue 1e+01)))

(event Input|AxisEvents|InputAxisMoveUpDown
  (params (AxisValue :type Float%20%28single-precision%29))
  ;[1 1 1] Movement Logic
  (Variables|Default|SetOffsetZ (* AxisValue 1e+01)))

(event Input|AxisEvents|InputAxisLookLeftRight
  (params (AxisValue :type Float%20%28single-precision%29))
  ;[1 1 1] Camera control
  (Pawn|Input|AddControllerYawInput AxisValue))

(event Input|AxisEvents|InputAxisLookUpDown
  (params (AxisValue :type Float%20%28single-precision%29))
  ;[1 1 1] Camera control
  (Pawn|Input|AddControllerPitchInput AxisValue))

(fn ConstructionScript
  (Transformation|SetRelativeRotation (Variables|Default|GetControlRig) (Variables|/Script/Engine.SceneComponent|GetRelativeRotation (Variables|Character|GetMesh)) false false))