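; Claw character that lets the player move a rig's control point along three axes.
; Input axes nudge the "Control" bone of a PoseableMesh in world X, Y and Z by a fixed step, without delta-time scaling.
; Before each Control Rig forward solve, that bone's transform is copied to Control_ctrl, with debug prints throughout.
; The construction script matches the Control Rig component's relative rotation to the mesh's.
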(event OnPreForwardsSolveDelegate(ControlRig)
  (params (Component :type Control%20Rig%20Component%20Object%20Reference))
  (bind _returnvalue (Class|PoseableMeshComponent|GetBoneTransformbyName (Variables|Default|GetPoseableMesh) "Control" "WorldSpace"))
  (Class|ControlRigComponent|SetControlTransform (Variables|Default|GetControlRig) "Control_ctrl" _returnvalue "WorldSpace")
  (Development|PrintString (Utilities|String|ToString(Transform) _returnvalue) true true "(R=1.000000,G=0.108477,B=0.756016,A=1.000000)"))

(event EventBeginPlay)

(event Collision|EventActorBeginOverlap
  (params (OtherActor :type Actor%20Object%20Reference)))

(event EventTick
  (params (DeltaSeconds :type Float%20%28single-precision%29)))

(event Input|AxisEvents|InputAxisMoveForwardBackward
  (params (AxisValue :type Float%20%28single-precision%29))
  (bind _poseablemesh (Variables|Default|GetPoseableMesh))
  (bind _returnvalue (Class|PoseableMeshComponent|GetBoneLocationbyName _poseablemesh "Control" "WorldSpace"))
  (Class|PoseableMeshComponent|SetBoneLocationbyName _poseablemesh "Control" (+ _returnvalue (Math|Vector|MakeVector (* AxisValue 1e+01) 0.0 0.0)) "WorldSpace")
  (Development|PrintString (Utilities|String|ToString(Vector) (+ _returnvalue (Math|Vector|MakeVector (* AxisValue 1e+01) 0.0 0.0)))))

(event Input|AxisEvents|InputAxisMoveLeftRight
  (params (AxisValue :type Float%20%28single-precision%29))
  (bind _poseablemesh (Variables|Default|GetPoseableMesh))
  (bind _returnvalue (Class|PoseableMeshComponent|GetBoneLocationbyName _poseablemesh "Control" "WorldSpace"))
  (Class|PoseableMeshComponent|SetBoneLocationbyName _poseablemesh "Control" (+ _returnvalue (Math|Vector|MakeVector 0.0 (* AxisValue 1e+01) 0.0)) "WorldSpace")
  (Development|PrintString (Utilities|String|ToString(Vector) (+ _returnvalue (Math|Vector|MakeVector 0.0 (* AxisValue 1e+01) 0.0))) true true "(R=1.000000,G=0.000000,B=0.000000,A=1.000000)"))

(event Input|AxisEvents|InputAxisMoveUpDown
  (params (AxisValue :type Float%20%28single-precision%29))
  (bind _poseablemesh (Variables|Default|GetPoseableMesh))
  (bind _returnvalue (Class|PoseableMeshComponent|GetBoneLocationbyName _poseablemesh "Control" "WorldSpace"))
  (Class|PoseableMeshComponent|SetBoneLocationbyName _poseablemesh "Control" (+ _returnvalue (Math|Vector|MakeVector 0.0 0.0 (* AxisValue 1e+01))) "WorldSpace")
  (Development|PrintString (Utilities|String|ToString(Vector) (+ _returnvalue (Math|Vector|MakeVector 0.0 0.0 (* AxisValue 1e+01)))) true true "(R=0.000000,G=1.000000,B=0.000000,A=1.000000)"))

(fn ConstructionScript
  (Transformation|SetRelativeRotation (Variables|Default|GetControlRig) (Variables|/Script/Engine.SceneComponent|GetRelativeRotation (Variables|Default|GetPoseableMesh)) false false))